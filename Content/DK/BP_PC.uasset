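; Player controller, judging by its name, that manages objective interactions in a killer-versus-survivor game: generators, hooks, pallets and the exit.
; On BeginPlay it finds these actors and binds their dispatchers, with Call functions forwarding to custom events.
; These events advance progress by delta time, set clear or play flags, drop hooks with physics, and destroy pallets after a delay, re-enabling Killer input.
; Generator clears increment a GameMode counter that lights the exit at a threshold.
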(event Custom|ClearGenerator
  (params (Target :type BP%20Generator%20Mul%20Object%20Reference))
  ;[1 1 1] 미션 클리어
  (if (Utilities|IsValid Target)
    (Variables|/Game/DK/BP_Generator_Mul.BP_Generator_Mul_C|SetbIsClear Target true)
    ;[1 1 1] 클리어 발전기 수 ++  , 클리어 조건 체크 후 탈출 위치 나타남.
    (bind _asdk_test_game_mode (Utilities|Casting|CastToDK_TestGameMode (Game|GetGameMode)))
    (bind _result (Math|Integer|IncrementInt (Variables|/Game/DK/DK_TestGameMode.DK_TestGameMode_C|GetCountClear _asdk_test_game_mode))
      (:%20%20
        (if (== _result 2)
          (Variables|/Game/DK/BP_ExitTest.BP_ExitTest_C|SetClearIntensity (Variables|Default|GetExit) 2e+01))))))

(event Custom|UpdateGenProgress
  (params (TargetP :type Float%20%28double-precision%29) (Target :type BP%20Generator%20Mul%20Object%20Reference))
  ;[1 1 1] 발전기 프로그래스바 업데이트
  (Variables|/Game/DK/BP_Generator_Mul.BP_Generator_Mul_C|SetRepairProgress Target (+ TargetP (Utilities|Time|GetWorldDeltaSeconds))))

(event Custom|ClearHook
  (params (Target :type BP%20Gal%20Progress%20Object%20Reference))
  ;[1 1 1] 후크 클리어
  (if (Utilities|IsValid Target)
    (Physics|SetSimulatePhysics (Variables|/Game/DK/BP_GalProgress.BP_GalProgress_C|GetSM_Hook Target) true)))

(event Custom|UpdateHookProgress
  (params (Target :type BP%20Gal%20Progress%20Object%20Reference) (Progress :type Float%20%28double-precision%29))
  ;[1 1 1] 후크 프로그래스바 업데이트
  (Variables|/Game/DK/BP_GalProgress.BP_GalProgress_C|SetRepairProgress Target (+ Progress (Utilities|Time|GetWorldDeltaSeconds))))

(event Custom|PalletPlay
  (params (Target :type BP%20Pallet%20Break%20Object%20Reference))
  (Variables|/Game/DK/BP_Pallet_Break.BP_Pallet_Break_C|SetbIsPalletPlay Target true))

(event Custom|UpdateExitProgress
  (bind _exit (Variables|Default|GetExit))
  ;[1 1 1] Comment
  (Variables|/Game/DK/BP_ExitTest.BP_ExitTest_C|SetExitProgress _exit (+ (Variables|/Game/DK/BP_ExitTest.BP_ExitTest_C|GetExitProgress _exit) (Utilities|Time|GetWorldDeltaSeconds))))

(event Custom|ClearExit
  (Variables|/Game/DK/BP_ExitTest.BP_ExitTest_C|SetbIsClear (Variables|Default|GetExit) true))

(event Custom|DestroyPallet
  (params (Target :type BP%20Pallet%20Break%20Object%20Reference))
  (bind _killer (Variables|/Game/DK/BP_Pallet_Break.BP_Pallet_Break_C|GetKiller Target))
  (Variables|/Game/DK/BP_Pallet_Break.BP_Pallet_Break_C|SetbIsPalletDestroy Target true)
  (Utilities|FlowControl|Delay 4.4)
  (if (Utilities|IsValid Target)
    (Input|EnableInput _killer (Pawn|GetLocalViewingPlayerController _killer))
    (Actor|DestroyActor Target)))

(event EventBeginPlay
  (Utilities|FlowControl|Sequence
    (:then_0
      ;[1 1 1] 발전기 바인딩
      (bind _outactors (Actor|GetAllActorsOfClass "/Game/DK/BP_Generator_Mul.BP_Generator_Mul_C"))
      (for _array_element _outactors
        (EventDispatchers|BindEventtoEDClear1 _array_element (EventDispatchers|CreateEvent :!event CallDestroy))
        (EventDispatchers|BindEventtoEDUpdateProgress _array_element (EventDispatchers|CreateEvent :!event CallProgress))))
    (:then_1
      ;[1 1 1] 갈고리 바인딩
      (bind _outactors_2 (Actor|GetAllActorsOfClass "/Game/DK/BP_GalProgress.BP_GalProgress_C"))
      (for _array_element_2 _outactors_2
        (EventDispatchers|BindEventtoEDUpdateGalProgress _array_element_2 (EventDispatchers|CreateEvent :!event CallGalProgress))
        (EventDispatchers|BindEventtoEDClearHook _array_element_2 (EventDispatchers|CreateEvent :!event CallClearHook))))
    (:then_2
      ;[1 1 1] 탈출구 지정
      (bind _outactors_3 (Actor|GetAllActorsOfClass "/Game/DK/BP_ExitTest.BP_ExitTest_C"))
      (bind _output_get (Variables|Default|SetExit (Utilities|Array|Get(acopy) _outactors_3)))
      (EventDispatchers|BindEventtoEDClearExit _output_get (EventDispatchers|CreateEvent :!event CallClearExit))
      (EventDispatchers|BindEventtoEDUdateExitProgress (Variables|Default|GetExit) (EventDispatchers|CreateEvent :!event CallUpdateExit)))
    (:then_3
      (bind _outactors_4 (Actor|GetAllActorsOfClass "/Game/DK/BP_Pallet_Break.BP_Pallet_Break_C"))
      (for _array_element_3 _outactors_4
        (EventDispatchers|BindEventtoEDPalletPlay _array_element_3 (EventDispatchers|CreateEvent :!event CallPalletPlay))
        (EventDispatchers|BindEventtoEDPalletDestroy _array_element_3 (EventDispatchers|CreateEvent :!event CallPalletDestroy))))))

(fn ConstructionScript)

(fn CallDestroy
  (params (Target :type BP%20Generator%20Mul%20Object%20Reference))
  (CallFunction|ClearGenerator Target))

(fn CallProgress
  (params (ServerProgress :type Float%20%28double-precision%29) (TargetGen :type BP%20Generator%20Mul%20Object%20Reference))
  (CallFunction|UpdateGenProgress ServerProgress TargetGen))

(fn CallGalProgress
  (params (Target :type BP%20Gal%20Progress%20Object%20Reference) (ServerProgressHook :type Float%20%28double-precision%29))
  (CallFunction|UpdateHookProgress Target ServerProgressHook))

(fn CallClearHook
  (params (TargetGen :type BP%20Gal%20Progress%20Object%20Reference))
  (CallFunction|ClearHook TargetGen))

(fn CallClearExit
  (CallFunction|ClearExit))

(fn CallUpdateExit
  (params (Progress :type Float%20%28double-precision%29) (Target :type BP%20Exit%20Test%20Object%20Reference))
  (CallFunction|UpdateExitProgress))

(fn CallPalletPlay
  (params (Target :type BP%20Pallet%20Break%20Object%20Reference))
  (CallFunction|PalletPlay Target))

(fn CallPalletDestroy
  (params (Target :type BP%20Pallet%20Break%20Object%20Reference))
  (CallFunction|DestroyPallet Target))