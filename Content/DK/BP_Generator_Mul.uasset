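; Multiplayer generator objective that survivors repair by holding an interact input inside its trigger box.
; Overlap by a locally controlled survivor enables input, adds a progress widget and opens a gate for the hold logic.
; Holding sends progress through event-dispatcher calls, and a retriggerable delay signals completion.
; RepNotifies refresh the widget and, on clear, play the looping generator animation; the minigame popup is never called here.
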(event OnComponentBeginOverlap(Box)
  (params (OverlappedComponent :type Primitive%20Component%20Object%20Reference) (OtherActor :type Actor%20Object%20Reference) (OtherComp :type Primitive%20Component%20Object%20Reference) (OtherBodyIndex :type Integer) (bFromSweep :type Boolean) (SweepResult :type Hit%20Result%20Structure%20%28by%20ref%29))
  ;[1 1 1] Mission Overlap 시 'E' 키 상호작용 설정
  (if (not (Variables|Default|GetbIsClear))
    (bind _asbp_test_survivor (Utilities|Casting|CastToBP_TestSurvivor OtherActor))
    (Variables|Default|SetCurrentPlayer _asbp_test_survivor)
    (if (Pawn|IsLocallyControlled (Variables|Default|GetCurrentPlayer))
      (Input|EnableInput (Pawn|GetLocalViewingPlayerController (Variables|Default|GetCurrentPlayer)))
      ;[1 1 1] Mission Overlap시 진행도 / 안내문구 Widget 설정
      (bind _returnvalue (Game|ConstructObjectfromClass "/Game/ThirdPerson/Blueprints/Survivor/Mission/WBP_MissionProgress.WBP_MissionProgress_C"))
      (bind _output_get (Variables|Default|SetWidgetREF _returnvalue))
      (UserInterface|Viewport|AddtoViewport _output_get 0)
      (Variables|/Game/ThirdPerson/Blueprints/Survivor/Mission/WBP_MissionProgress.WBP_MissionProgress_C|SetTimeHeld _output_get (- (Variables|Default|GetMaxHeldTime) (Variables|Default|GetRepairProgress)))
      (Variables|/Game/ThirdPerson/Blueprints/Survivor/Mission/WBP_MissionProgress.WBP_MissionProgress_C|SetMaxTimeHeld _output_get (Variables|Default|GetMaxHeldTime))
      ;[1 1 1] Mission Progress Bar
      (Utilities|FlowControl|Gate true) ; enters at Open
    )))

(event OnComponentEndOverlap(Box)
  (params (OverlappedComponent :type Primitive%20Component%20Object%20Reference) (OtherActor :type Actor%20Object%20Reference) (OtherComp :type Primitive%20Component%20Object%20Reference) (OtherBodyIndex :type Integer))
  ;[1 1 1] Mission Overlap 시 'E' 키 상호작용 설정
  (bind _asbp_test_survivor (Utilities|Casting|CastToBP_TestSurvivor OtherActor))
  (Variables|Default|SetCurrentPlayer _asbp_test_survivor)
  (if (Pawn|IsLocallyControlled (Variables|Default|GetCurrentPlayer))
    (Input|DisableInput (Pawn|GetLocalViewingPlayerController (Variables|Default|GetCurrentPlayer)))
    ;[1 1 1] Mission Overlap시 진행도 / 안내문구 Widget 설정
    (Variables|Default|SetIsHeld false)
    (bind _widgetref (Variables|Default|GetWidgetREF)
      (:then
        (Widget|RemovefromParent _widgetref)
        ;[1 1 1] Mission Progress Bar
        (Utilities|FlowControl|Gate true) ; enters at Close
      )
      (:else))))

(event Custom|Timer
  ;[1 1 1] Mission Progress Bar 시간 설정
  (bind _returnvalue (Utilities|Time|SetTimerbyEvent (delegate Custom|Timer) (Variables|Default|GetMaxHeldTime) false false 0.01)))

(event Custom|Stop%20Timer
  ;[1 1 1] Mission Progress Bar 시간 설정
  (Utilities|Time|PauseTimerbyHandle (stale Custom|Timer _returnvalue)))

(event Custom|Update%20Timer
  (bind _repairprogress (Variables|Default|GetRepairProgress))
  (bind _maxheldtime (Variables|Default|GetMaxHeldTime))
  (bind _returnvalue (- _maxheldtime _repairprogress))
  ;[1 1 1] Mission Progress Bar 시간 설정
  (if (Variables|Default|GetIsHeld)
    (Variables|/Game/ThirdPerson/Blueprints/Survivor/Mission/WBP_MissionProgress.WBP_MissionProgress_C|SetTimeHeld (Variables|Default|GetWidgetREF) _returnvalue)
    (Utilities|FlowControl|Delay 0.01)
    (CallFunction|UpdateTimer)
    (else
      (CallFunction|StopTimer)
      (Variables|/Game/ThirdPerson/Blueprints/Survivor/Mission/WBP_MissionProgress.WBP_MissionProgress_C|SetTimeHeld (Variables|Default|GetWidgetREF) _returnvalue))))

(event Input|EnhancedActionEvents|EnhancedInputActionIA_Live_Trigger
  (params (ActionValue :type Boolean) (ElapsedSeconds :type Float%20%28double-precision%29) (TriggeredSeconds :type Float%20%28double-precision%29) (InputAction :type Input%20Action%20Object%20Reference :default "/Game/Create/GM/Input/Survivor/IA_Live_Trigger.IA_Live_Trigger"))
  (:Triggered
    (if (Variables|Default|GetIsHeld)
      (Default|CallEDUpdateProgress (Variables|Default|GetRepairProgress) self)))
  (:Started
    (Variables|Default|SetIsHeld true)
    (if (not (Variables|Default|GetbIsClear))
      ;[1 1 1] Mission Progress Bar
      (Utilities|FlowControl|Gate true
        (:Exit
          (Utilities|FlowControl|Sequence
            (:then_0
              (Utilities|FlowControl|RetriggerableDelay (- (Variables|Default|GetMaxHeldTime) (Variables|Default|GetRepairProgress)))
              (if (Variables|Default|GetIsHeld)
                (Default|CallEDClear1 self)))
            (:then_1
              (CallFunction|Timer)
              (CallFunction|UpdateTimer)))))))
  (:Completed
    (Variables|Default|SetIsHeld false)
    (Utilities|Time|PauseTimerbyHandle)))

(fn ConstructionScript)

(fn MiniGame
  (if (>= (Variables|Default|GetRepairProgress) 1.0)
    (Utilities|FlowControl|DoOnce false
      (:Completed
        (bind _returnvalue (UserInterface|CreateWidget "/Game/ThirdPerson/Blueprints/Survivor/MiniGame/WBP_MiniGame.WBP_MiniGame_C"))
        (UserInterface|Viewport|AddtoViewport _returnvalue 0)))))

(fn OnRepBIsClear
  (Components|Animation|PlayAnimation (Variables|Default|GetSKM_Generator) "/Game/Create/Mesh/SKM/Generator/Anim_SKM_Generator.Anim_SKM_Generator" true)
  (bind _widgetref (Variables|Default|GetWidgetREF)
    (:then
      (Widget|RemovefromParent _widgetref))
    (:else)))

(fn OnRepRepairProgress
  (bind _widgetref (Variables|Default|GetWidgetREF)
    (:then
      (Variables|/Game/ThirdPerson/Blueprints/Survivor/Mission/WBP_MissionProgress.WBP_MissionProgress_C|SetTimeHeld _widgetref (- (Variables|Default|GetMaxHeldTime) (Variables|Default|GetRepairProgress))))
    (:else)))