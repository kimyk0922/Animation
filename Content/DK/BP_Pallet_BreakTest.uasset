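; Breakable pallet for a two-player Survivor versus Killer game: the Survivor drops it and the Killer destroys it.
; Box overlaps show per-player trigger widgets and open gates for each role's input; the Survivor's tilts PalletBone via timeline.
; Once dropped, the Killer's input plays a destroy montage with input disabled, then destroys the actor.
; Two-stage functions, uncalled here, enable physics on piece groups for staged breakage.
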(event OnComponentBeginOverlap(Box)
  (params (OverlappedComponent :type Primitive%20Component%20Object%20Reference) (OtherActor :type Actor%20Object%20Reference) (OtherComp :type Primitive%20Component%20Object%20Reference) (OtherBodyIndex :type Integer) (bFromSweep :type Boolean) (SweepResult :type Hit%20Result%20Structure%20%28by%20ref%29))
  (bind _returnvalue (Game|GetPlayerController 0))
  ;[0 0.2 0 0.5 15] Surviver
  (bind _asbp_survivor (Utilities|Casting|CastToBP_Survivor OtherActor)
    (:then
      (Variables|/Game/Create/GM/BP_Survivor.BP_Survivor_C|SetCurrPallet _asbp_survivor 0)
      (bind _returnvalue_2 (UserInterface|CreateWidget "/Game/Create/Blueprint/WG_Trigger_Info.WG_Trigger_Info_C"))
      (UserInterface|Viewport|AddtoPlayerScreen _returnvalue_2 1)
      (Utilities|FlowControl|Gate true) ; enters at Open
    )
    (:CastFailed
      (if (Variables|Default|GetbIsPalletPlay)
        ;[0.2 0 0 0.5 15] Killer
        (bind _asbp_killer (Utilities|Casting|CastToBP_Killer OtherActor))
        (bind _output_get (Variables|Default|SetKiller _asbp_killer))
        (Variables|/Game/Create/GM/BP_Killer.BP_Killer_C|SetCurrPallet _output_get 0)
        (bind _returnvalue_3 (UserInterface|CreateWidget "/Game/Create/Blueprint/WG_Trigger_Info.WG_Trigger_Info_C"))
        (UserInterface|Viewport|AddtoPlayerScreen _returnvalue_3)
        (Utilities|FlowControl|Gate true) ; enters at Open
      ))))

(event OnComponentEndOverlap(Box)
  (params (OverlappedComponent :type Primitive%20Component%20Object%20Reference) (OtherActor :type Actor%20Object%20Reference) (OtherComp :type Primitive%20Component%20Object%20Reference) (OtherBodyIndex :type Integer))
  (bind _returnvalue (Game|GetPlayerController 0))
  (bind _killer (Variables|Default|GetKiller))
  ;[0 0.2 0 0.5 15] Surviver
  (Utilities|Casting|CastToBP_Survivor OtherActor
    (:then
      (Widget|RemovefromParent (stale OnComponentBeginOverlap(Box) _returnvalue_2))
      (Utilities|FlowControl|Gate true) ; enters at Close
    )
    (:CastFailed
      ;[0.2 0 0 0.5 15] Killer
      (if (Variables|Default|GetbIsPalletPlay)
        (Utilities|Casting|CastToBP_Killer OtherActor)
        (Widget|RemovefromParent (stale OnComponentBeginOverlap(Box) _returnvalue_3))
        (Utilities|FlowControl|Gate true) ; enters at Close
      ))))

(event Input|EnhancedActionEvents|EnhancedInputActionIA_Killer_Trigger
  (params (ActionValue :type Boolean) (ElapsedSeconds :type Float%20%28double-precision%29) (TriggeredSeconds :type Float%20%28double-precision%29) (InputAction :type Input%20Action%20Object%20Reference :default "/Game/Create/GM/Input/Killer/IA_Killer_Trigger.IA_Killer_Trigger"))
  (bind _returnvalue (Game|GetPlayerController 0))
  (bind _killer (Variables|Default|GetKiller))
  ;[0.2 0 0 0.5 15] Killer
  (:Started
    (Utilities|FlowControl|Gate true
      (:Exit
        (Animation|Montage|PlayMontage (Variables|/Script/Engine.Character|GetMesh (stale OnComponentBeginOverlap(Box) _output_get)) "/Game/Create/Animation/Killer/Anim_Destroy.Anim_Destroy"
          (:then
            (Input|DisableInput _killer _returnvalue))
          (:OnCompleted
            (Input|EnableInput _killer _returnvalue)
            (Actor|DestroyActor)))))))

(event Input|EnhancedActionEvents|EnhancedInputActionIA_Live_Trigger
  (params (ActionValue :type Boolean) (ElapsedSeconds :type Float%20%28double-precision%29) (TriggeredSeconds :type Float%20%28double-precision%29) (InputAction :type Input%20Action%20Object%20Reference :default "/Game/Create/GM/Input/Survivor/IA_Live_Trigger.IA_Live_Trigger"))
  ;[0 0.2 0 0.5 15] Surviver
  (:Started
    (Utilities|FlowControl|Gate true
      (:Exit
        (bind _movespeed (Timeline|PalletMotion Play)
          (:Update
            (Transformation|SetRelativeRotation (Variables|Default|GetPallet_Bone) (Math|Rotator|MakeRotator 0.0 (Math|Float|Lerp 0.0 45.0 _movespeed) 0.0) false false)
            (Variables|Default|SetbIsPalletPlay true)))))))

(event EventBeginPlay
  ;[0.2 0 0 0.5 15] Killer
  (Input|EnableInput (Game|GetPlayerController 0))
  (Input|EnableInput (Game|GetPlayerController 1)))

(fn ConstructionScript)

(fn SimulatePhysics
  (params (bSimulate :type Boolean))
  (for _array_element (Components|GetChildrenComponents (Variables|/Game/Create/Blueprint/BP_Pallet_Break.BP_Pallet_Break_C|GetBox (Variables|Default|GetPallet)) false)
    (bind _asstatic_mesh_component (Utilities|Casting|CastToStaticMeshComponent _array_element))
    (Physics|SetSimulatePhysics _asstatic_mesh_component bSimulate)))

(fn SetPhysicsSecondTarget
  (Physics|SetSimulatePhysics (Variables|Default|GetPallet_Sphere_024) true))

(fn SetDestroySecondAction
  (CallFunction|SetPhysicsSecondTarget))

(fn SetDestroyFirstAction
  (CallFunction|SetPhysicsFirstTarget))

(fn SetPhysicsFirstTarget
  (Physics|SetSimulatePhysics (Variables|Default|GetPallet_Cube_044) true))