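; BP_Box is an interactable box that a BP_Survivor can open while standing inside its overlap volume.
; Overlap begin shows a WG_Trigger_Info prompt and opens a gate; overlap end removes the prompt and closes the gate.
; The box enables input on BeginPlay, so IA_Live_Trigger passes through the gate to play a timeline pitching SMBoxU from 0 to 90 degrees.
; No logic reverses the opening.
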(event OnComponentBeginOverlap(Box)
  (params (OverlappedComponent :type Primitive%20Component%20Object%20Reference) (OtherActor :type Actor%20Object%20Reference) (OtherComp :type Primitive%20Component%20Object%20Reference) (OtherBodyIndex :type Integer) (bFromSweep :type Boolean) (SweepResult :type Hit%20Result%20Structure%20%28by%20ref%29))
  (Utilities|Casting|CastToBP_Survivor OtherActor)
  (bind _returnvalue (UserInterface|CreateWidget "/Game/Create/Blueprint/WG_Trigger_Info.WG_Trigger_Info_C"))
  (UserInterface|Viewport|AddtoPlayerScreen _returnvalue)
  (Utilities|FlowControl|Gate true) ; enters at Open
)

(event OnComponentEndOverlap(Box)
  (params (OverlappedComponent :type Primitive%20Component%20Object%20Reference) (OtherActor :type Actor%20Object%20Reference) (OtherComp :type Primitive%20Component%20Object%20Reference) (OtherBodyIndex :type Integer))
  (Utilities|Casting|CastToBP_Survivor OtherActor)
  (Widget|RemovefromParent (stale OnComponentBeginOverlap(Box) _returnvalue))
  (Utilities|FlowControl|Gate true) ; enters at Close
)

(event Input|EnhancedActionEvents|EnhancedInputActionIA_Live_Trigger
  (params (ActionValue :type Boolean) (ElapsedSeconds :type Float%20%28double-precision%29) (TriggeredSeconds :type Float%20%28double-precision%29) (InputAction :type Input%20Action%20Object%20Reference :default "/Game/Create/GM/Input/Survivor/IA_Live_Trigger.IA_Live_Trigger"))
  (Utilities|FlowControl|Gate true
    (:Exit
      (bind _opentime (Timeline|Timeline Play)
        (:Update
          (Transformation|SetRelativeRotation (Variables|Default|GetSM_Box_U) (Math|Rotator|MakeRotator 0.0 (Math|Float|Lerp 0.0 9e+01 _opentime) 0.0) false false))))))

(event EventBeginPlay
  (Input|EnableInput (Game|GetPlayerController 0)))

(fn ConstructionScript)